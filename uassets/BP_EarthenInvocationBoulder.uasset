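; Boulder actor for Earthen Invocation that forms with effects matched to a surface type, then rises beside gameplay logic driven by its instigator.
; Initialisation sinks it by its bounds radius, then sets the Niagara formation effect's material and dust colour per surface, disabling smoke for metal.
; A timeline raises it to a height scaled from the caster's taller skeletal mesh bounds, then signals completion through a dispatcher component that is exposed with the material.
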(event EventInitialiseBoulder
  (params (_surfaceType :type EEarthenInvocationSupportedSurfaces%20Enum :default "NewEnumerator0"))
  (CallFunction|InitialiseLocation)
  (CallFunction|InitialiseVFX _surfaceType)
  (Rendering|SetVisibility (Actor|GetComponentbyClass "/Script/Engine.SceneComponent") true true))

(event EventRaiseBoulder
  (bind _returnvalue (Transformation|GetActorLocation))
  (bind _instigator (Variables|Actor|GetInstigator))
  (bind _returnvalue_2 (Actor|GetComponentbyClass _instigator "/Script/Engine.SkeletalMeshComponent"))
  (bind _returnvalue_3 (Actor|GetComponentsbyTag _instigator "/Script/Engine.SkeletalMeshComponent" "Body"))
  (bind _output (Utilities|Array|Get(acopy) _returnvalue_3))
  (bind _skeletalmeshasset (Variables|/Script/Engine.SkeletalMeshComponent|GetSkeletalMeshAsset _returnvalue_2))
  (bind _returnvalue_4 (StaticMesh|GetBounds _skeletalmeshasset))
  (bind _skeletalmeshasset_2 (Variables|/Script/Engine.SkeletalMeshComponent|GetSkeletalMeshAsset _output))
  (bind _returnvalue_5 (StaticMesh|GetBounds _skeletalmeshasset_2))
  (Variables|Default|SetinitialHeight (.z (Transformation|GetActorLocation)))
  (bind _output_get (Variables|Default|SetmaximumHeight (+ (* (select (> (.z (.boxextent _returnvalue_4)) (.z (.boxextent _returnvalue_5))) (.z (.boxextent _returnvalue_4)) (.z (.boxextent _returnvalue_5))) (Variables|Default|GetmaximumHeightMultiplierRelativeToCaster)) (Variables|/Script/Engine.SphereComponent|GetSphereRadius (Variables|Default|GetBounds)))))
  (bind _raiseoffset (Timeline|RaiseTimeline PlayFromStart)
    (:Update
      (Transformation|SetActorLocation (Math|Vector|MakeVector (.x _returnvalue) (.y _returnvalue) (+ (* _raiseoffset _output_get) (Variables|Default|GetinitialHeight))) false true))
    (:Finished
      (Default|CallAnimationComplete (Variables|Default|GetBPC_EarthenInvocationDispatcher)))))

(fn ConstructionScript
  (Niagara|SetNiagaraVariable(Float) (Variables|Default|GetBoulder%20Formation%20VFX) "_radius" (Variables|/Script/Engine.SphereComponent|GetSphereRadius (Variables|Default|GetBounds))))

(fn InitialiseLocation
  (bind _returnvalue (Transformation|GetActorLocation))
  (Transformation|SetActorLocation (Math|Vector|MakeVector (.x _returnvalue) (.y _returnvalue) (- (.z _returnvalue) (Variables|/Script/Engine.SphereComponent|GetSphereRadius (Variables|Default|GetBounds)))) false true))

(fn InitialiseVFX
  (params (surfaceType :type EEarthenInvocationSupportedSurfaces%20Enum :default "NewEnumerator0"))
  (switch Utilities|FlowControl|Switch|SwitchonEEarthenInvocationSupportedSurfaces surfaceType
    (:NewEnumerator0
      (Variables|Default|Setmaterial "/Game/Samsara/Blueprints/Actions/Spells/Mantras/EarthenInvocation/VFX/Boulder/Materials/MI_Stone.MI_Stone" :!label _label)
      ;[1 1 1] Default (grey smoke)
      (Niagara|SetNiagaraVariable(LinearColor) (Variables|Default|GetBoulder%20Formation%20VFX) "_dustColour" (Utilities|Struct|MakeLinearColor 0.75 0.75 0.75 1.0)))
    (:NewEnumerator1
      (Variables|Default|Setmaterial "/Game/Samsara/Blueprints/Actions/Spells/Mantras/EarthenInvocation/VFX/Boulder/Materials/MI_Dirt.MI_Dirt" :!label _label_2)
      ;[1 1 1] Brown smoke
      (Niagara|SetNiagaraVariable(LinearColor) (Variables|Default|GetBoulder%20Formation%20VFX) "_dustColour" (Utilities|Struct|MakeLinearColor 0.3 0.2 0.15 1.0)))
    (:NewEnumerator2
      (goto _label_2))
    (:NewEnumerator3
      (goto _label_2))
    (:NewEnumerator4
      (goto _label))
    (:NewEnumerator5
      (Variables|Default|Setmaterial "/Game/Samsara/Blueprints/Actions/Spells/Mantras/EarthenInvocation/VFX/Boulder/Materials/MI_Metal.MI_Metal")
      ;[1 1 1] Transparent (no smoke)
      (Effects|Components|ParticleSystem|SetEmitterEnable (Variables|Default|GetBoulder%20Formation%20VFX) "Smoke" false))
    (:NewEnumerator6
      (Variables|Default|Setmaterial "/Game/Samsara/Blueprints/Actions/Spells/Mantras/EarthenInvocation/VFX/Boulder/Materials/MI_Snow.MI_Snow")
      ;[1 1 1] White smoke
      (Niagara|SetNiagaraVariable(LinearColor) (Variables|Default|GetBoulder%20Formation%20VFX) "_dustColour" (Class|KismetMathLibrary|LinearColorWhite)))
    (:NewEnumerator7
      (Variables|Default|Setmaterial "/Game/Samsara/Blueprints/Actions/Spells/Mantras/EarthenInvocation/VFX/Boulder/Materials/MI_Sand.MI_Sand")
      ;[1 1 1] Yellow smoke
      (Niagara|SetNiagaraVariable(LinearColor) (Variables|Default|GetBoulder%20Formation%20VFX) "_dustColour" (Utilities|Struct|MakeLinearColor 0.8 0.72 0.5 1.0))))
  (Class|NiagaraComponent|SetVariableMaterial (Variables|Default|GetBoulder%20Formation%20VFX) "_boulderMaterial" (Variables|Default|Getmaterial))
  (Components|Activation|Activate (Variables|Default|GetBoulder%20Formation%20VFX) false))

(fn GetBoulderDispatcher
  (return (Variables|Default|GetBPC_EarthenInvocationDispatcher)))

(fn GetBoulderMaterial
  (return (Variables|Default|Getmaterial)))