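; Manager actor for the Earthen Invocation spell that replaces a boulder with a spread of projectiles along the spell direction.
; Projectiles spawn within the boulder's sphere bounds with its material, and their hits apply earth and poise damage to enemies.
; A timer scaled by the instigator's Wisdom ends remaining projectiles, using a map to skip those already despawning.
; Despawns go through BPI_EarthenInvocation, and the manager destroys itself once the map empties.
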(event Custom|Event%20StopTimer
  (Utilities|Time|ClearandInvalidateTimerbyHandle (stale EventBeginPlay _returnvalue_2)))

(event Custom|Event%20OnDestroy
  (params (DestroyedActor :type Actor%20Object%20Reference))
  ;[1 1 1] Projectile Destroy Event.  Handles the destruction of the manager when all projectiles have been destroyed.
  (Utilities|Map|Remove (Variables|Default|Getprojectiles) DestroyedActor)
  (if (Utilities|Map|IsEmpty (Variables|Default|Getprojectiles))
    (Actor|DestroyActor)))

(event Custom|Event%20OnHit
  (params (SelfActor :type Actor%20Object%20Reference) (OtherActor :type Actor%20Object%20Reference) (NormalImpulse :type Vector) (Hit :type Hit%20Result%20Structure%20%28by%20ref%29))
  ;[1 1 1] Projectile hit event. This is invoked when a blocking collision is detected on the projectile. Handles damage application to enemies and triggers despawning the projectile.
  (bind _returnvalue (Class|EarthenInvocationManager|AreActorsEnemies OtherActor (Game|GetInstigator SelfActor)))
  (if _returnvalue
    (Class|EarthenInvocationManager|ApplyDamage OtherActor (Variables|Default|GetearthDamage) (Variables|Default|GetpoiseDamage) (Variables|Default|GetdamageReduceScale) "/Game/Samsara/Blueprints/Core/DamageTypes/BP_EarthDamageType.BP_EarthDamageType_C" "/Game/Samsara/Blueprints/Core/DamageTypes/BP_PoiseDamageType.BP_PoiseDamageType_C"))
  (if (Utilities|Map|Contains (Variables|Default|Getprojectiles) 0)
    (Utilities|Map|Add (Variables|Default|Getprojectiles) SelfActor false))
  (if (Utilities|DoesObjectImplementInterface SelfActor "/Game/Samsara/Blueprints/Actions/Spells/Mantras/EarthenInvocation/BPI_EarthenInvocation.BPI_EarthenInvocation_C")
    (Class|BPIEarthenInvocation|PrepareDestroy(Message) SelfActor)
    (else
      (Actor|DestroyActor SelfActor))))

(event Custom|Event%20DestroyRemainingProjectiles
  ;[1 1 1] Projectile lifetime has elapsed, so destroy all projectiles that haven't already been destroyed/started their destruction.
  (CallFunction|EventStopTimer)
  (bind _keys (Utilities|Map|Keys (Variables|Default|Getprojectiles)))
  (for _array_element _keys
    (if (.Value (Utilities|Map|Find (Variables|Default|Getprojectiles) _array_element))
      (if (Utilities|DoesObjectImplementInterface _array_element "/Game/Samsara/Blueprints/Actions/Spells/Mantras/EarthenInvocation/BPI_EarthenInvocation.BPI_EarthenInvocation_C")
        (Class|BPIEarthenInvocation|PrepareDestroy(Message) _array_element)
        (else
          (Actor|DestroyActor _array_element))))))

(event EventBeginPlay
  (bind _projectilelifespan (Variables|Default|GetprojectileLifespan))
  (bind _boulder (Variables|Default|Getboulder))
  (bind _returnvalue (Actor|GetComponentbyClass _boulder "/Script/Engine.SphereComponent"))
  (bind (_origin _boxextent) (Collision|GetComponentBounds _returnvalue))
  (Utilities|FlowControl|DelayUntilNextTick)
  (bind _material (Class|BPIEarthenInvocation|GetBoulderMaterial(Message) (Variables|Default|Getboulder)))
  (Class|EarthenInvocationManager|SpawnProjectiles "/Game/Samsara/Blueprints/Actions/Spells/Mantras/EarthenInvocation/BP_EarthenInvocationProjectile.BP_EarthenInvocationProjectile_C" (Variables|Default|GetnumberOfProjectiles) _origin _boxextent (Variables|Default|GetspellDirection) (Variables|Default|GetprojectileSpread) _material (Math|Conversions|ToVector(Float) 0.85))
  (Actor|DestroyActor (Variables|Default|Getboulder))
  (bind _keys (Utilities|Map|Keys (Variables|Default|Getprojectiles)))
  (for _array_element _keys
    (Collision|BindEventtoOnActorHit _array_element (delegate Custom|Event%20OnHit))
    (Game|BindEventtoOnDestroyed _array_element (delegate Custom|Event%20OnDestroy)))
  ;[1 1 1] Scales projectile lifetime (the spell's range) proportionally with with the player's WISDOM.
  (bind _wisdomscale (CallFunction|GetNormalisedWisdom 6 50))
  (bind _returnvalue_2 (Utilities|Time|SetTimerbyEvent (delegate Custom|Event%20DestroyRemainingProjectiles) (+ _projectilelifespan (* _projectilelifespan (* _wisdomscale (/ (Variables|Default|GetprojectileLifespanMaxPercentageIncrease) 1e+02)))))))

(event EventInitialiseManager
  (params (_direction :type Vector :default "0, 0, 0") (_numberOfProjectiles :type Integer) (_boulder :type Actor%20Object%20Reference%20%28by%20ref%29) (_earthDamage :type Float%20%28double-precision%29) (_poiseDamage :type Float%20%28double-precision%29) (_projectileLifespan :type Float%20%28double-precision%29) (_projectileLifespanMaxPercentageIncrease :type Float%20%28double-precision%29))
  (Variables|Default|SetspellDirection _direction)
  (Variables|Default|SetnumberOfProjectiles _numberOfProjectiles)
  (Variables|Default|Setboulder _boulder)
  (Variables|Default|SetearthDamage _earthDamage)
  (Variables|Default|SetpoiseDamage _poiseDamage)
  (Variables|Default|SetprojectileLifespan _projectileLifespan)
  (Variables|Default|SetprojectileLifespanMaxPercentageIncrease _projectileLifespanMaxPercentageIncrease))

(fn ConstructionScript)

(fn GetNormalisedWisdom
  (params (_minLevel :type Integer) (_maxLevel :type Integer))
  (bind _instigator (Variables|Default|GetInstigator))
  (bind _returnvalue (Actor|GetComponentbyClass _instigator "/Script/AdvancedRPGSystem.ARSStatisticsComponent"))
  (Utilities|IsValid _returnvalue
    (:Is%20Valid
      (bind _output_get (LocalVariables|Setlevel (Math|Float|Truncate (Class|ARSStatisticsComponent|GetCurrentPrimaryAttributeValue _returnvalue "(TagName=\"RPG.PrimaryAttributes.Wisdom\")"))))
      (if (<= _output_get _minLevel)
        (return 0.0)
        (elif (>= (LocalVariables|Getlevel) _maxLevel)
          (return 1.0)
          (else
            (return (/ (- (LocalVariables|Getlevel) _minLevel) (- _maxLevel _minLevel)))))))
    (:Is%20Not%20Valid
      (return 0.0))))

(fn GetBoulderDispatcher
  (return 0))

(fn GetBoulderMaterial
  (return 0))