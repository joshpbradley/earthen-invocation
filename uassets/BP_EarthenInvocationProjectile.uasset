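; Projectile actor for Earthen Invocation, with a sphere collider, static mesh, projectile movement and Niagara trail.
; On spawn, the sphere ignores its instigator while moving so it does not hit the firing pawn.
; PrepareDestroy ignores Pawn collision, stops movement and trail emission, then a timeline fades the trail and shrinks the mesh before destroying the actor.
; The boulder dispatcher and material getters are empty stubs.
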(event EventBeginPlay
  ;[1 1 1] Prevents projectiles from colliding with the pawn that is firing the projectiles.
  (Collision|IgnoreActorwhenMoving (Variables|Components|GetCollisionSphere) (Game|GetInstigator) true))

(event EventPrepareDestroy
  ;[1 1 1] Disables collision and movement, then gracefully fades/shrinks the projectile before destruction.
  (Collision|SetCollisionResponsetoChannel (Variables|Components|GetCollisionSphere) "ECC_Pawn" "ECR_Ignore")
  (Components|Activation|Deactivate (Variables|Components|GetProjectileMovement))
  (Effects|Components|ParticleSystem|SetEmitterEnable (Variables|Components|GetTrail) "Trail" false)
  (Variables|Default|SetinitialScale (Transformation|GetWorldScale (Variables|Components|GetStaticMesh)))
  (bind (_direction _alpha _scale) (Timeline|Fade%20Trail%20and%20Shrink%20Projectile PlayFromStart)
    (:Update
      (Niagara|SetNiagaraVariable(Float) (Variables|Components|GetTrail) "_alpha" _alpha)
      (Transformation|SetWorldScale3D (Variables|Components|GetStaticMesh) (* (Variables|Default|GetinitialScale) _scale)))
    (:Finished
      (Actor|DestroyActor))))

(fn ConstructionScript)

(fn GetBoulderDispatcher
  (return 0))

(fn GetBoulderMaterial
  (return 0))